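; Behavior tree service that finds the nearest player character for the AI pawn on each service tick.
; It scans all BP_PlayerCharacter actors, filters them through IsValidAndAlive, and keeps the closest by distance.
; It writes that actor to the TargetToFollow blackboard key and the distance to DistToTarget.
; With no match, TargetToFollow is left unchanged and DistToTarget receives a huge sentinel value.
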(event `self.ReceiveTickAI`
  (params (OwnerController :type "AIController Object Reference") (ControlledPawn :type "Pawn Object Reference") (DeltaSeconds :type "Float (single-precision)"))
  (set `self.ClosestDistance` 99999997952.0)
  (set `self.ControlledActor` ControlledPawn)
  (bind _outactors (`GameplayStatics.GetAllActorsOfClass` "/Game/Blueprints/BP_PlayerCharacter.BP_PlayerCharacter_C"))
  (for _array_element _outactors
    (bind (_asbp_character _bsuccess) (cast `/Game/Blueprints/BP_Character` _array_element :!pure true))
    (if (and (`/Game/Blueprints/BP_Character.IsAlive` _asbp_character) (`KismetSystemLibrary.IsValid` _asbp_character) _bsuccess)
      (bind _returnvalue (`Actor.GetDistanceTo` (`self.ControlledActor`) _array_element))
      (if (< _returnvalue (`self.ClosestDistance`))
        (set `self.ClosestDistance` _returnvalue)
        (`BTFunctionLibrary.SetBlackboardValueAsObject` (`self.TargetToFollow`) _array_element))))
  (`BTFunctionLibrary.SetBlackboardValueAsFloat` (`self.DistToTarget`) (`self.ClosestDistance`)))