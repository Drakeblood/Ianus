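; Animation notify that deals boss sphere attack damage to the player at a point in the animation.
; It runs a Pawn sphere overlap at the mesh component's world location plus an unrotated offset, using a configurable radius.
; Overlapped actors that cast to BP_PlayerCharacter receive the GE_BossHandAttackDamage gameplay effect through their Ability System Component.
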(fn `Received_Notify`
  (params (MeshComp :type "SkeletalMeshComponent Object Reference") (Animation :type "AnimSequenceBase Object Reference"))
  (returns (ReturnValue :type Boolean))
  (bind _outactors (`KismetSystemLibrary.SphereOverlapActors` (+ (`SceneComponent.K2_GetComponentLocation` MeshComp) (`self.OffsetLocation`)) (`self.SphereRadius`) (`|MakeArray` "ObjectTypeQuery3" :!type "EObjectTypeQuery Enum")))
  (for _array_element _outactors
    (bind _asbp_player_character (cast `/Game/Blueprints/BP_PlayerCharacter` _array_element))
    (`AbilitySystemComponent.BP_ApplyGameplayEffectToSelf` :`self` (`AbilitySystemBlueprintLibrary.GetAbilitySystemComponent` _asbp_player_character) :`GameplayEffectClass` "/Game/Blueprints/GameplayEffects/GE_BossHandAttackDamage.GE_BossHandAttackDamage_C" :`Level` 1.0))
  (return true))