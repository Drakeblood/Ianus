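; Character Blueprint that provides health checks and skill and melee attack commands through the Gameplay Ability System.
; Attacks are gated on being alive, unpaused and not already using a skill, with active abilities detected by gameplay tag.
; Skills activate by tag and fire an attack notification, while melee activates the ability in the current weapon slot unless a melee is already running.
; A DelayedDestroy event destroys the actor.
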(event `DelayedDestroy`
  (`self.K2_DestroyActor`))

(fn `CanUseAnyAbility`
  (returns (Result :type Boolean))
  (return (and (`self.IsAlive`) (not (`GameplayStatics.IsGamePaused`)) (not (`self.IsUsingSkill`)))))

(fn `DoMeleeAttack`
  (returns (ReturnValue :type Boolean))
  (if (and (`self.CanUseAnyAbility`) (not (`self.IsUsingMelee`)))
    (bind _returnvalue (`self.ActivateAbilitiesWithItemSlot` (`self.CurrentWeaponSlot`) :!pinned true)) ; Melee attack command, uses weapon slots
    (return _returnvalue)))

(fn `DoSkillAttack`
  (returns (ReturnValue :type Boolean))
  (if (`self.CanUseAnyAbility`)
    (bind _returnvalue (`self.ActivateAbilitiesWithTags` (struct :`GameplayTags` (struct :`(TagName` "Ability.Skill")))))
    (`self.OnSkillAttack`)
    (return _returnvalue)))

(fn `IsAlive`
  (returns (Return :type Boolean))
  (return (> (`self.GetHealth`) 0.0)))

(fn `IsUsingMelee`
  (returns (Result :type Boolean))
  (bind _activeabilities (`self.GetActiveAbilitiesWithTags` (struct :`GameplayTags` (struct :`(TagName` "Ability.Melee")))))
  (return (> (`KismetArrayLibrary.Array_Length` _activeabilities) 0)))

(fn `IsUsingSkill`
  (returns (Result :type Boolean))
  (bind _activeabilities (`self.GetActiveAbilitiesWithTags` (struct :`GameplayTags` (struct :`(TagName` "Ability.Skill")))))
  (return (> (`KismetArrayLibrary.Array_Length` _activeabilities) 0)))

(fn `UserConstructionScript`)