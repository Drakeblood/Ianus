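; Behavior tree task that makes an AI-controlled IanusCharacterBase use a gameplay ability of a given class.
; It activates the class through the pawn's ability system component, then looks up active abilities matching the configured gameplay tags.
; It binds to the end event of the first match, cast to GA_Base, and finishes successfully only when that fires.
; A failed cast leaves the task without a finish call.
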(event `AbilityEnded`
  (`self.FinishExecute` true))

(event `self.ReceiveExecuteAI`
  (params (OwnerController :type "AIController Object Reference") (ControlledPawn :type "Pawn Object Reference"))
  (bind _asianus_character_base (cast `IanusCharacterBase` ControlledPawn))
  (`AbilitySystemComponent.TryActivateAbilityByClass` (`AbilitySystemBlueprintLibrary.GetAbilitySystemComponent` _asianus_character_base) (`self.GAClass`) true)
  (bind _activeabilities (`IanusCharacterBase.GetActiveAbilitiesWithTags` _asianus_character_base (`self.GameplayAbilityTags`)))
  (bind _asga_base (cast `/Game/Blueprints/GameplayAbilities/GA_Base` (`|GetArrayItem` _activeabilities)))
  (add `/Game/Blueprints/GameplayAbilities/GA_Base.OnAbilityEnded` _asga_base (delegate `AbilityEnded`)))