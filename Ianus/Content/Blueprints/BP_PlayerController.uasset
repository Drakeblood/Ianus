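; Player controller that relays attack input and weapon-slot changes to the controlled BP_PlayerCharacter.
; The NormalAttack press triggers the character's melee attack.
; On first possession only, a DoOnce and short delay precede setting game-only input and creating all of the character's weapons.
; SlottedItemChanged rebuilds those weapons whenever the changed slot's item type is Weapon.
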(event `InputAction|NormalAttack`
  (params (Key :type "Key Structure"))
  (bind _returnvalue (`self.K2_GetPawn`))
  (:`Pressed`
    (`/Engine/EditorBlueprintResources/StandardMacros.IsValid` _returnvalue
      (:`Is Valid`
        (bind _asbp_player_character (cast `/Game/Blueprints/BP_PlayerCharacter` _returnvalue))
        (`/Game/Blueprints/BP_Character.DoMeleeAttack` _asbp_player_character)))))

(event `self.ReceivePossess`
  (params (PossessedPawn :type "Pawn Object Reference"))
  (`/Engine/EditorBlueprintResources/StandardMacros.DoOnce` false
    (:`Completed`
      (`KismetSystemLibrary.Delay` 0.025)
      (`WidgetBlueprintLibrary.SetInputMode_GameOnly` self)
      (bind _asbp_player_character (cast `/Game/Blueprints/BP_PlayerCharacter` PossessedPawn))
      (`/Game/Blueprints/BP_PlayerCharacter.CreateAllWeapons` _asbp_player_character) ; Equip weapons
    )))

(event `self.SlottedItemChanged`
  (params (ItemSlot :type "IanusItemSlot Structure") (Item :type "IanusItemBase Object Reference"))
  (switch `name` (`.Name` (break `PrimaryAssetType` (`.ItemType` (break `IanusItemSlot` ItemSlot))))
    (:`Weapon`
      (bind _asbp_player_character (cast `/Game/Blueprints/BP_PlayerCharacter` (`self.K2_GetPawn`)))
      (`/Game/Blueprints/BP_PlayerCharacter.CreateAllWeapons` _asbp_player_character))))

(fn `UserConstructionScript`)